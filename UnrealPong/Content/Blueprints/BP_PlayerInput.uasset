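; BP_PlayerInput handles the Pause input action, toggling game pause and the pause menu.
; When unpaused, it creates a new WBP_PauseMenu, adds it to the viewport, pauses the game, and switches to game-and-UI input with the cursor shown.
; When paused, it removes that stored widget, restores game-only input, hides the cursor and unpauses.
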(event Input|ActionEvents|InputActionPause
  (params (Key :type Key%20Structure :default "None"))
  (bind _returnvalue (Game|GetPlayerController 0))
  (bind _returnvalue_2 (Game|GetPlayerController 0))
  (:Pressed
    (if (Game|IsGamePaused)
      (Widget|RemovefromParent (stale _returnvalue_3))
      (Input|SetInputModeGameOnly _returnvalue_2)
      (Variables|/Script/Engine.PlayerController|SetbShowMouseCursor _returnvalue_2 false)
      (Game|SetGamePaused false)
      (else
        (bind _returnvalue_3 (UserInterface|CreateWidget "/Game/Blueprints/Widgets/WBP_PauseMenu.WBP_PauseMenu_C"))
        (UserInterface|Viewport|AddtoViewport _returnvalue_3 0)
        (Game|SetGamePaused true)
        (Input|SetInputModeGameandUI _returnvalue 0 "DoNotLock" true)
        (Variables|/Script/Engine.PlayerController|SetbShowMouseCursor _returnvalue true)))))