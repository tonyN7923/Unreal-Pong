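; Game mode for a Pong game that detects when a player wins and ends the match.
; On BeginPlay it binds OnGoal to the reporter of every BP_Goal.
; Each goal triggers a check of every goal's player score against WinningScore.
; On a match it stores the winner's name, shows the cursor with UI-only input, destroys the ball and calls GameEndReporter.
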(event Custom|OnGoal
  (bind _returnvalue (Game|GetPlayerController 0))
  (bind _outactors (Actor|GetAllActorsOfClass "/Game/Blueprints/BP_Goal.BP_Goal_C"))
  (for _array_element _outactors
    (if (== (Variables|/Game/Blueprints/BP_Paddle.BP_Paddle_C|GetScore (Variables|/Game/Blueprints/BP_Goal.BP_Goal_C|GetPlayer _array_element)) (Variables|Default|GetWinningScore))
      (Variables|Default|SetWinnerName (Variables|/Game/Blueprints/BP_Paddle.BP_Paddle_C|GetName (Variables|/Game/Blueprints/BP_Goal.BP_Goal_C|GetPlayer _array_element)))
      (Variables|/Script/Engine.PlayerController|SetbShowMouseCursor _returnvalue true)
      (Input|SetInputModeUIOnly _returnvalue 0 "DoNotLock")
      (bind _returnvalue_2 (Actor|GetActorOfClass "/Game/Blueprints/BP_Ball.BP_Ball_C"))
      (Actor|DestroyActor _returnvalue_2)
      (Default|CallGameEndReporter))))

(event EventBeginPlay
  (bind _outactors (Actor|GetAllActorsOfClass "/Game/Blueprints/BP_Goal.BP_Goal_C"))
  (for _array_element _outactors
    (EventDispatchers|BindEventtoGoalReporter _array_element (delegate Custom|OnGoal))))

(fn ConstructionScript)