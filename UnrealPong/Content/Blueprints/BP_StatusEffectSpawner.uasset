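; BP_StatusEffectSpawner is an actor that randomly spawns status effect pickups or actors inside a box volume.
; Each Tick it rolls against SpawnChance, so the spawn rate depends on frame rate, and on success spawns a random class from Effects at a random point within the Box bounds.
; RemoveAllEffects stops and destroys every BP_StatusEffect in the world, not only those this spawner created.
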(event EventTick
  (params (DeltaSeconds :type Float%20%28single-precision%29))
  (if (Math|Random|RandomBoolwithWeight (Variables|Default|GetSpawnChance))
    (CallFunction|SpawnRandomEffect)))

(fn ConstructionScript)

(fn GetRandomSpawnLocation
  (bind _box (Variables|Default|GetBox))
  (bind (_origin _boxextent) (Collision|GetComponentBounds _box))
  (return (Math|Random|RandomPointinBoundingBox _origin _boxextent)))

(fn SpawnRandomEffect
  (bind _newparam (CallFunction|GetRandomEffect))
  (bind _location (CallFunction|GetRandomSpawnLocation))
  (Game|SpawnActorfromClass _newparam (Math|Transform|MakeTransform _location) "Undefined" 0 0))

(fn GetRandomEffect
  (return (.OutItem (Utilities|Array|Random (Variables|Default|GetEffects)))))

(fn RemoveAllEffects
  (bind _outactors (Actor|GetAllActorsOfClass "/Game/Blueprints/BP_StatusEffect.BP_StatusEffect_C"))
  (for _array_element _outactors
    (Default|StopEffect _array_element)
    (Actor|DestroyActor _array_element)))