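; BP_PaddleHalfSize is a status effect that halves the size of a player's paddle along its X axis.
; ApplyEffect finds BP_Ball, stores its LastHitByPlayer as the affected player and divides that actor's X scale by two.
; StopEffect, if that player is still valid, sets a hardcoded uniform scale of 0.5 rather than restoring a saved original.
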(event EventApplyEffect
  (bind _returnvalue (Actor|GetActorOfClass "/Game/Blueprints/BP_Ball.BP_Ball_C"))
  (bind _output_get (Variables|Default|SetPlayerAffected (Variables|/Game/Blueprints/BP_Ball.BP_Ball_C|GetLastHitByPlayer _returnvalue)))
  (Transformation|SetActorScale3D _output_get (Math|Vector|MakeVector (/ (.X (Math|Vector|BreakVector (Transformation|GetActorScale3D (Variables|Default|GetPlayerAffected)))) 2.0) (.Y (Math|Vector|BreakVector (Transformation|GetActorScale3D (Variables|Default|GetPlayerAffected)))) (.Z (Math|Vector|BreakVector (Transformation|GetActorScale3D (Variables|Default|GetPlayerAffected)))))))

(event EventStopEffect
  (bind _playeraffected (Variables|Default|GetPlayerAffected)
    (:then
      (Transformation|SetActorScale3D _playeraffected "0.500000,0.500000,0.500000"))
    (:else)))

(fn ConstructionScript
  (|CallParentFunction))