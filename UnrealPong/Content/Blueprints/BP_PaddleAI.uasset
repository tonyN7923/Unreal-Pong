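; BP_PaddleAI is a computer-controlled paddle that follows the ball along the X axis.
; Each tick, after the parent tick, AIMove finds a BP_Ball actor with GetActorOfClass and compares its X position to the paddle's own.
; Offsets beyond MoveThreshold become a signed unit input and smaller ones become zero, a dead zone applied before calling Move.
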(event EventTick
  (params (DeltaSeconds :type Float%20%28single-precision%29))
  (|CallParentFunction DeltaSeconds)
  (CallFunction|AIMove DeltaSeconds))

(fn ConstructionScript
  (|CallParentFunction))

(fn AIMove
  (params (Delta%20Seconds :type Float%20%28double-precision%29))
  (bind _returnvalue (Actor|GetActorOfClass "/Game/Blueprints/BP_Ball.BP_Ball_C"))
  (if (Utilities|IsValid _returnvalue)
    (bind _output_get (LocalVariables|SetDeltaPosition (- (.X (Math|Vector|BreakVector (Transformation|GetActorLocation _returnvalue))) (.X (Math|Vector|BreakVector (Transformation|GetActorLocation))))))
    (if (> (Math|Float|Absolute(Float) _output_get) (Variables|Default|GetMoveThreshold))
      (LocalVariables|SetDeltaPosition (Math|Float|Sign(Float) (LocalVariables|GetDeltaPosition)))
      (else
        (bind _output_get_2 (LocalVariables|SetDeltaPosition 0.0))))
    (CallFunction|Move _output_get_2 Delta%20Seconds)))