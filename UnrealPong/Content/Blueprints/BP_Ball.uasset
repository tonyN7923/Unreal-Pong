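; Physics-driven ball that launches along positive or negative Y at random and plays a sound cue on hits.
; While simulating, Tick adds impulses whenever total speed drops below MinSpeed or Y speed below MinSpeed/√2, keeping the ball moving along Y.
; Reset plays a dissolve effect, returns the ball to a fixed center point with physics and trail off, then relaunches it after a short delay.
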(event OnComponentHit(SphereCollision)
  (params (HitComponent :type Primitive%20Component%20Object%20Reference) (OtherActor :type Actor%20Object%20Reference) (OtherComp :type Primitive%20Component%20Object%20Reference) (NormalImpulse :type Vector :default "0, 0, 0") (Hit :type Hit%20Result%20Structure%20%28by%20ref%29))
  (if (not (Audio|Components|Audio|IsPlaying (Variables|Default|GetS_Ball_Hit_Cue)))
    (Audio|Components|Audio|Play (Variables|Default|GetS_Ball_Hit_Cue) 0.0)))

(event Custom|Reset
  (Components|Activation|SetActive (Variables|Default|GetDissolve) true false)
  (Utilities|FlowControl|Delay 1.0)
  (Components|Activation|SetActive (Variables|Default|GetDissolve) false false)
  (Components|Activation|SetActive (Variables|Default|GetTrail) false false)
  (Transformation|SetActorLocation "0, 0,100.000000" false false)
  (CallFunction|SimulateBallMovement false)
  (Utilities|FlowControl|Delay 1.0)
  (CallFunction|GetRandomVelocity)
  (CallFunction|SimulateBallMovement true)
  (Components|Activation|SetActive (Variables|Default|GetTrail) true false))

(event EventBeginPlay
  (CallFunction|GetRandomVelocity)
  (Components|Activation|SetActive (Variables|Default|GetDissolve) false false))

(event EventTick
  (params (DeltaSeconds :type Float%20%28single-precision%29))
  (if (Physics|IsSimulatingPhysics (Variables|Default|GetSphereCollision) "None")
    (CallFunction|AdjustHorizontalVelocity)
    (CallFunction|AdjustVelocity)))

(fn ConstructionScript)

(fn SimulateBallMovement
  (params (Simulate :type Boolean))
  (Physics|SetSimulatePhysics (Variables|Default|GetSphereCollision) Simulate))

(fn GetRandomVelocity
  (if (Math|Random|RandomBool)
    (LocalVariables|SetVelocity "0,-1.000000, 0")
    (else
      (LocalVariables|SetVelocity "0,1.000000, 0")))
  (Physics|SetPhysicsLinearVelocity (Variables|Default|GetSphereCollision) (* (LocalVariables|GetVelocity) (Variables|Default|GetMinSpeed)) false "None"))

(fn IsSpeedAboveMinimum
  (return (>= (Math|Vector|VectorLength (Transformation|GetComponentVelocity (Variables|Default|GetSphereCollision))) (Variables|Default|GetMinSpeed))))

(fn AdjustVelocity
  (bind _result (CallFunction|IsSpeedAboveMinimum))
  (if (not _result)
    (bind _velocity (CallFunction|GetMinimumHorizontalVelocity))
    (Physics|AddImpulse (Variables|Default|GetSphereCollision) (* _velocity (Math|Vector|Normalize (Transformation|GetComponentVelocity (Variables|Default|GetSphereCollision)))) "None" false)))

(fn AdjustHorizontalVelocity
  (bind _spherecollision (Variables|Default|GetSphereCollision))
  (bind _returnvalue (Transformation|GetComponentVelocity _spherecollision))
  (bind _returnvalue_2 (Math|Vector|Normalize _returnvalue))
  (bind (_x _y _z) (Math|Vector|BreakVector _returnvalue_2))
  (bind _result (CallFunction|IsHorizontalVelocityAboveMinimum))
  (if (not _result)
    (bind _velocity (CallFunction|GetMinimumHorizontalVelocity))
    (Physics|AddImpulse (Variables|Default|GetSphereCollision) (Math|Vector|MakeVector _x (* _velocity _y) _z) "None" false)))

(fn IsHorizontalVelocityAboveMinimum
  (bind _velocity (CallFunction|GetMinimumHorizontalVelocity))
  (return (>= (Math|Float|Absolute(Float) (.Y (Math|Vector|BreakVector (Transformation|GetComponentVelocity (Variables|Default|GetSphereCollision))))) _velocity)))

(fn GetMinimumHorizontalVelocity
  (return (/ (Variables|Default|GetMinSpeed) (Math|Float|Sqrt 2.0))))